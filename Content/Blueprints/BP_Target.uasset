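; BP_Target is a moving shooting target that awards the player points when hit by a projectile.
; On BeginPlay it stores the VRPawn, then two chained timelines endlessly lerp it between its spawn location and a fixed Y position.
; Head and Body overlaps with a Projectile add points to the pawn, more for the head, and play distinct sounds.
; An unconnected destroy-and-game-mode-score branch never runs.
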(event OnComponentBeginOverlap(Head)
  (params (OverlappedComponent :type Primitive%20Component%20Object%20Reference) (OtherActor :type Actor%20Object%20Reference) (OtherComp :type Primitive%20Component%20Object%20Reference) (OtherBodyIndex :type Integer) (bFromSweep :type Boolean) (SweepResult :type Hit%20Result%20Structure%20%28by%20ref%29))
  (bind _characterref (Variables|Default|GetCharacterRef))
  (Utilities|Casting|CastToProjectile OtherActor)
  (Variables|/Game/VRTemplate/Blueprints/VRPawn.VRPawn_C|SetPoints _characterref (+ (Variables|/Game/VRTemplate/Blueprints/VRPawn.VRPawn_C|GetPoints _characterref) 20))
  (Audio|PlaySoundatLocation "/Game/Sounds/368298__radioactive_blueberry__slap.368298__radioactive_blueberry__slap" (Transformation|GetActorLocation) "0, 0, 0" 1.0 1.0 0.0 0 0 0 0))

(event OnComponentBeginOverlap(Body)
  (params (OverlappedComponent :type Primitive%20Component%20Object%20Reference) (OtherActor :type Actor%20Object%20Reference) (OtherComp :type Primitive%20Component%20Object%20Reference) (OtherBodyIndex :type Integer) (bFromSweep :type Boolean) (SweepResult :type Hit%20Result%20Structure%20%28by%20ref%29))
  (bind _characterref (Variables|Default|GetCharacterRef))
  (Utilities|Casting|CastToProjectile OtherActor)
  (Variables|/Game/VRTemplate/Blueprints/VRPawn.VRPawn_C|SetPoints _characterref (+ (Variables|/Game/VRTemplate/Blueprints/VRPawn.VRPawn_C|GetPoints _characterref) 10))
  (Audio|PlaySoundatLocation "/Game/Sounds/9933__davepape__boink-0010.9933__davepape__boink-0010" (Transformation|GetActorLocation) "0, 0, 0" 1.0 1.0 0.0 0 0 0 0))

(event EventBeginPlay
  (bind _returnvalue (Transformation|GetActorLocation))
  (Variables|Default|SetStart (Math|Vector|MakeVector (.x _returnvalue) (.y _returnvalue) (.z _returnvalue)))
  (Variables|Default|SetEnd (Math|Vector|MakeVector (.x _returnvalue) -1.42e+03 (.z _returnvalue)))
  (bind _asvrpawn (Utilities|Casting|CastToVRPawn (Game|Player|GetPlayerPawn 0)))
  (Variables|Default|SetCharacterRef _asvrpawn)
  (bind _move (Timeline|Move PlayFromStart)
    (:Update
      (Transformation|SetActorRelativeLocation (Math|Vector|Lerp(Vector) (Variables|Default|GetStart) (Variables|Default|GetEnd) _move)))
    (:Finished
      (bind _move_2 (Timeline|Move%20Back ReverseFromEnd)
        (:Update
          (Transformation|SetActorRelativeLocation (Math|Vector|Lerp(Vector) (Variables|Default|GetStart) (Variables|Default|GetEnd) _move_2)))
        (:Finished
          (Timeline|Move PlayFromStart))))))

(fn ConstructionScript)